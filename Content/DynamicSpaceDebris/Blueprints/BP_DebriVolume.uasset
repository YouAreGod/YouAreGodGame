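; Debris volume actor that scatters randomized mesh instances inside a sphere, cube or cylinder and can animate them.
; The construction script creates one instanced static mesh component per debris type, then places objects with randomized transforms, retrying locations that overlap other debris or BP_DebrisBlockingVolume.
; Optional radius spheres visualize each object's spacing.
; When enabled, Tick applies spin plus optional center pivot or wrapping Z-axis movement, dirtying render state once per component.
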(event `self.ReceiveTick`
  (params (DeltaSeconds :type "Float (single-precision)"))
  ;[1 1 1] Do not run unless needed
  (if (and (`self.Update Transforms`) (`self.Active`))
    ;[1 1 1] Loop through each object instance spawned
    (for (_array_element _array_index) (`self.Debris ISM`)
      (bind _returnvalue (- (`InstancedStaticMeshComponent.GetInstanceCount` _array_element) 1))
      (for _index (range (+ _returnvalue 1))
        (bind _returnvalue_2 (`KismetMathLibrary.MakeTransform` (.location (`InstancedStaticMeshComponent.GetInstanceTransform` _array_element _index false)) (`KismetMathLibrary.ComposeRotators` (.rotation (`InstancedStaticMeshComponent.GetInstanceTransform` _array_element _index false)) (* (`.RotationRate_38_13A63D564875D5A2F4A72B86194DEE2E` (break `/Game/DynamicSpaceDebris/Blueprints/Structures/BPS_DebrisVolume` (`KismetArrayLibrary.Array_Get` (`self.Object Instances`) _array_index))) (`GameplayStatics.GetWorldDeltaSeconds`))) (.scale (`InstancedStaticMeshComponent.GetInstanceTransform` _array_element _index false))))
        (bind _location (.location _returnvalue_2))
        (bind (_minimumscale _maximumscale _minimumrotation _maximumrotation _minimumdistance _maximumdistance _centerpitch _centeryaw) (break `/Game/DynamicSpaceDebris/Blueprints/Structures/BPS_DebrisVolume` (`KismetArrayLibrary.Array_Get` (`self.Object Instances`) _array_index)))
        (bind _location_2 (.location _returnvalue_2))
        (bind _returnvalue_3 (`self.Unlocalize Vector Rotation` _location_2))
        ;[1 1 1] Update instance transforms
        (`InstancedStaticMeshComponent.UpdateInstanceTransform` _array_element _index (select `/Game/DynamicSpaceDebris/Blueprints/Structures/Enum_DebrisMovement` (`self.Movement Type`) :`NewEnumerator0` _returnvalue_2 :`NewEnumerator1` (`KismetMathLibrary.MakeTransform` (`self.Localize Vector Rotation` (`KismetMathLibrary.GreaterGreater_VectorRotator` (`self.Unlocalize Vector Rotation` _location) (`KismetMathLibrary.MakeRotator` (.x (* (`self.Object Velocity`) (`GameplayStatics.GetWorldDeltaSeconds`))) (.y (* (`self.Object Velocity`) (`GameplayStatics.GetWorldDeltaSeconds`))) (.z (* (`self.Object Velocity`) (`GameplayStatics.GetWorldDeltaSeconds`)))))) (`KismetMathLibrary.MakeRotator` (.roll (.rotation _returnvalue_2)) (select `bool` _centerpitch :`false` (.pitch (.rotation _returnvalue_2)) :`true` (.pitch (`KismetMathLibrary.FindLookAtRotation` _location (`KismetMathLibrary.MakeVector` 0.0)))) (select `bool` _centeryaw :`false` (.yaw (.rotation _returnvalue_2)) :`true` (.yaw (`KismetMathLibrary.FindLookAtRotation` _location (`KismetMathLibrary.MakeVector` 0.0))))) (.scale _returnvalue_2)) :`NewEnumerator2` (`KismetMathLibrary.MakeTransform` (select `bool` (< (.z (* (`self.GetActorScale3D`) 50)) (.z _returnvalue_3)) :`false` (+ (* (`self.Localize Vector Rotation` (`self.Object Velocity`)) (`GameplayStatics.GetWorldDeltaSeconds`)) _location_2) :`true` (`self.Localize Vector Rotation` (`KismetMathLibrary.MakeVector` (.x _returnvalue_3) (.y _returnvalue_3) (* -1 (.z _returnvalue_3))))) (.rotation _returnvalue_2) (.scale _returnvalue_2))) false (== _index _returnvalue) false)))))

(fn `UserConstructionScript`
  (locals (`Random Spawn Value` :type "Float (double-precision)"))
  (bind _object_velocity (`self.Object Velocity`))
  (bind _volume_shape (`self.Volume Shape`))
  (bind _volume_shape_2 (`self.Volume Shape`))
  ;[1 1 1] Spawn debris
  (bind _returnvalue (`PrimitiveComponent.CreateDynamicMaterialInstance` (`self.Volume`) 0 "/Game/DynamicSpaceDebris/Materials/M_Debris_Volume.M_Debris_Volume"))
  (`MaterialInstanceDynamic.SetVectorParameterValue` _returnvalue "Color" (`self.Volume Color`))
  (bind _returnvalue_2 (`PrimitiveComponent.CreateDynamicMaterialInstance` (`self.Debris Radius Display`) 0 "/Game/DynamicSpaceDebris/Materials/M_Debris_Volume.M_Debris_Volume"))
  (`MaterialInstanceDynamic.SetVectorParameterValue` _returnvalue_2 "Color" (`self.Object Radius Color`))
  (set `self.Volume Shape` (select `/Game/DynamicSpaceDebris/Blueprints/Structures/Enum_DebrisMovement` (`self.Movement Type`) :`NewEnumerator0` _volume_shape :`NewEnumerator1` _volume_shape :`NewEnumerator2` (select `bool` (`|EnumEquality` _volume_shape_2 "NewEnumerator0") :`false` _volume_shape_2 :`true` "NewEnumerator2")))
  (`StaticMeshComponent.SetStaticMesh` (`self.Volume`) (select `/Game/DynamicSpaceDebris/Blueprints/Structures/Enum_DebrisVolumeShape` _volume_shape :`NewEnumerator0` "/Engine/BasicShapes/Sphere.Sphere" :`NewEnumerator2` "/Engine/BasicShapes/Cube.Cube" :`NewEnumerator1` "/Engine/BasicShapes/Cylinder.Cylinder" :!type "StaticMesh Object Reference"))
  (for _array_element (`self.Object Instances`)
    (bind _returnvalue_3 (`AddComponent|NODE_AddInstancedStaticMeshComponent-0`))
    (`PrimitiveComponent.SetCastShadow` _returnvalue_3 (`self.Cast Shadows`))
    (`KismetArrayLibrary.Array_Add` (`self.Debris ISM`) _returnvalue_3) ; Add the components to an array for referencing
    (bind (_minimumscale _maximumscale _minimumrotation _maximumrotation _minimumdistance _maximumdistance _centerpitch _centeryaw _mesh _materialinstance) (break `/Game/DynamicSpaceDebris/Blueprints/Structures/BPS_DebrisVolume` _array_element))
    (`StaticMeshComponent.SetStaticMesh` _returnvalue_3 _mesh)
    (`PrimitiveComponent.SetMaterial` _returnvalue_3 0 _materialinstance)
    (`SceneComponent.SetAbsolute` _returnvalue_3 false true true)
    (`SceneComponent.SetAbsolute` (`self.Debris Radius Display`) false true true))
  (set `self.Object Velocity` (select `bool` (`|EnumEquality` (`self.Movement Type`) "NewEnumerator2") :`false` _object_velocity :`true` (`KismetMathLibrary.MakeVector` 0.0 0.0 (.z _object_velocity))))
  (if (`self.Active`)
    (for _ (range 1 (+ (`self.Object Count`) 1))
      _)))