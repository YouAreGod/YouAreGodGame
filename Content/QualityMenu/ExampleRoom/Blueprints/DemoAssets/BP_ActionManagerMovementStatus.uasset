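; Demo actor for the QualityMenu example room that displays live movement and look axis values as text.
; ActionManager axis events for forward, right, look up and look right each store their value in a variable.
; The Update Keybinding input axis event serves as the update loop, manually ticking the ActionManager and then writing the four stored values into the Text component.
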(event `self.ActionManager.MoveForward`
  (params (Axis :type "Float (single-precision)"))
  (set `self.Forward Value` Axis))

(event `self.ActionManager.MoveRight`
  (params (Axis :type "Float (single-precision)"))
  (set `self.Right Value` Axis))

(event `self.ActionManager.LookUp`
  (params (Axis :type "Float (single-precision)"))
  (set `self.LookUp` Axis))

(event `self.ActionManager.LookRight`
  (params (Axis :type "Float (single-precision)"))
  (set `self.LookRight` Axis))

(event `InputAxis|Update Keybinding`
  (params (AxisValue :type "Float (single-precision)"))
  (`/Game/QualityMenu/Blueprints/BP_ActionManager.Tick Action Manager` (`self.ActionManager`))
  (`TextRenderComponent.K2_SetText` (`self.Text`) (`KismetTextLibrary.Conv_StringToText` (`KismetStringLibrary.Concat_StrStr` "Forward Axis: " (`KismetStringLibrary.Conv_DoubleToString` (`self.Forward Value`)) " \n" "Right Axis: " (`KismetStringLibrary.Conv_DoubleToString` (`self.Right Value`)) " \n" "Look Up: " (`KismetStringLibrary.Conv_DoubleToString` (`self.LookUp`)) " \n" "Look Right: " (`KismetStringLibrary.Conv_DoubleToString` (`self.LookRight`))))))

(fn `UserConstructionScript`)