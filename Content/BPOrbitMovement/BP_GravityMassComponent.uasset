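; Gravity source component that computes the acceleration its owning actor exerts on an orbiting object passed to GravityAccelerationExerted.
; Pull is the gravitational parameter over squared distance, clamped by a minimum, toward the actor's origin or closest point on its static meshes.
; An optional reverse line trace detects being inside the owner and adds pull from the opposite surface to temper gravity.
; Options disable the effect, restrict it to the interior, or invert it as anti-gravity.
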(fn `GravityAccelerationExerted`
  (params (TheOrbit :type "/Game/BPOrbitMovement/Lib/BP_Orbit Object Reference"))
  (returns (GravAccelerationExerted :type "Vector Structure"))
  (locals (GravityVector :type "Vector Structure") (GravityMassLocation :type "Vector Structure") (TheOtherOrbit :type "/Game/BPOrbitMovement/Lib/BP_Orbit Object Reference") (OtherActorLocation :type "Vector Structure") (isInside :type Boolean))
  (bind _otheractorlocation (`local.OtherActorLocation`))
  (bind _otheractorlocation_2 (`local.OtherActorLocation`))
  (bind _returnvalue (`Actor.K2_GetComponentsByClass` (`self.GetOwner`) "/Script/Engine.StaticMeshComponent"))
  (bind _returnvalue_2 (`KismetArrayLibrary.Array_Length` _returnvalue))
  (bind _returnvalue_3 (- (`local.GravityMassLocation`) (`Actor.K2_GetActorLocation` (`/Game/BPOrbitMovement/Lib/BP_Orbit.ParentActor` (`local.TheOtherOrbit`)))))
  (bind _returnvalue_4 (- (`local.GravityMassLocation`) (`Actor.K2_GetActorLocation` (`/Game/BPOrbitMovement/Lib/BP_Orbit.ParentActor` (`local.TheOtherOrbit`)))))
  (if (`self.bWillAffectGravity`)
    (set `local.TheOtherOrbit` TheOrbit)
    (set `local.OtherActorLocation` (`Actor.K2_GetActorLocation` (`/Game/BPOrbitMovement/Lib/BP_Orbit.ParentActor` (`local.TheOtherOrbit`))))
    (if (`self.bUseClosestPointOnStaticMesh`)
      ;[1 1 1] Find the closest point on the staticmesh to the orbiting actor. Use that to base the gravitational distance
      (set `local.GravityMassLocation` (`PrimitiveComponent.GetClosestPointOnCollision` (`KismetArrayLibrary.Array_Get` _returnvalue) (`local.OtherActorLocation`) "None"))
      ;[1 1 1] Loop through all staticmesh actors to find the closest point on any staticmesh actor
      (if (> _returnvalue_2 1)
        (for _index (range 1 _returnvalue_2)
          (bind _outpointonbody (`PrimitiveComponent.GetClosestPointOnCollision` (`KismetArrayLibrary.Array_Get` _returnvalue _index) (`local.OtherActorLocation`) "None"))
          (if (< (`KismetMathLibrary.VSizeSquared` (- _otheractorlocation _outpointonbody)) (`KismetMathLibrary.VSizeSquared` (- (`local.GravityMassLocation`) _otheractorlocation)))
            (set `local.GravityMassLocation` _outpointonbody))))
      (else
        (set `local.GravityMassLocation` (`Actor.K2_GetActorLocation` (`self.GetOwner`)))))
    (set `local.GravityVector` (* (`/Game/BPOrbitMovement/Lib/BP_Orbit.UnsafeNormal` (`local.TheOtherOrbit`) _returnvalue_3) (/ (`self.StandardGravitationalParameter`) (`KismetMathLibrary.FMax` (`KismetMathLibrary.VSizeSquared` _returnvalue_3) (`self.MinDistanceForKinematicGravity`)))))
    ;[1 1 1] For traveling inside objects, gravity may vary too much if it only calculates gravity from one point. This checks the opposite direction of the closest point and tempers gravity
    (if (`self.CheckGravityForInsideObject`)
      (bind (_outhit _returnvalue_5) (`KismetSystemLibrary.LineTraceSingleForObjects` :`Start` _otheractorlocation_2 :`End` (+ _otheractorlocation_2 (* (`local.GravityVector`) -100000.0)) :`ObjectTypes` (`|MakeArray` "ObjectTypeQuery1" "ObjectTypeQuery2" "ObjectTypeQuery4" :!type "EObjectTypeQuery Enum") :`bIgnoreSelf` false))
      ;;[1 1 1] No hit
      (if _returnvalue_5
        (bind (_bblockinghit _binitialoverlap _time _location _impactpoint _normal _impactnormal _physmat _hitactor) (`GameplayStatics.BreakHitResult` _outhit))
        ;;[1 1 1] Not the same actor as the GravityMass owner
        (if (== _hitactor (`self.GetOwner`))
          (set `local.GravityMassLocation` _location)
          (set `local.GravityVector` (+ (* (`/Game/BPOrbitMovement/Lib/BP_Orbit.UnsafeNormal` (`local.TheOtherOrbit`) _returnvalue_4) (/ (`self.StandardGravitationalParameter`) (`KismetMathLibrary.FMax` (`KismetMathLibrary.VSizeSquared` _returnvalue_4) (`self.MinDistanceForKinematicGravity`)))) (`local.GravityVector`)))
          (set `local.isInside` true))))
    (if (and (not (`local.isInside`)) (`self.bOnlyAffectIfInsideOwner`))
      (return (0.0 0.0 0.0))
      (else
        ;[1 1 1] Reverse gravity if Anti-gravity option is selected.
        (if (`self.bAntiGravity`)
          (set `local.GravityVector` (* (`local.GravityVector`) -1.0)))
        (return (`local.GravityVector`))))
    (else
      (return (0.0 0.0 0.0)))))