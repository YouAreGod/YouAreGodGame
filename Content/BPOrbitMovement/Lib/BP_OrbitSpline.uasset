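; BP_OrbitSpline is a spline actor in the orbit movement library that can render its path with static meshes.
; DrawStaticMeshes adds a spline mesh component per spline point, attaches it to Scene and bends a thinly scaled SplineStaticMesh to the next point using local locations and tangents.
; The construction script and events are empty, so nothing in this graph calls DrawStaticMeshes.
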(event EventBeginPlay)

(event EventActorBeginOverlap
  (params (OtherActor :type Actor%20Object%20Reference)))

(event EventTick
  (params (DeltaSeconds :type Float%20%28single-precision%29)))

(fn ConstructionScript)

(fn DrawStaticMeshes
  (bind _spline (Variables|Default|GetSpline))
  (for _index (range 0 (- (Spline|GetNumberOfSplinePoints (Variables|Default|GetSpline)) 1))
    (bind _returnvalue (AddComponent|AddSplineMeshComponent true))
    (LocalVariables|SetTempSplineMesh _returnvalue)
    (Components|StaticMesh|SetStaticMesh (LocalVariables|GetTempSplineMesh) (Variables|Default|GetSplineStaticMesh))
    (SplineMesh|SetEndScale (LocalVariables|GetTempSplineMesh) "(X=0.200000,Y=0.200000)" :!class /Script/Engine.SplineMeshComponent)
    (SplineMesh|SetStartScale (LocalVariables|GetTempSplineMesh) "(X=0.200000,Y=0.200000)" :!class /Script/Engine.SplineMeshComponent)
    (Class|SceneComponent|Attachto (LocalVariables|GetTempSplineMesh) (Variables|Default|GetScene) "None" "KeepRelativeOffset" true)
    (SplineMesh|SetStartandEnd (LocalVariables|GetTempSplineMesh) (.Location (Spline|GetLocationandTangentatSplinePoint _spline _index "Local")) (.Tangent (Spline|GetLocationandTangentatSplinePoint _spline _index "Local")) (.Location (Spline|GetLocationandTangentatSplinePoint _spline (+ _index 1) "Local")) (.Tangent (Spline|GetLocationandTangentatSplinePoint _spline (+ _index 1) "Local")) :!class /Script/Engine.SplineMeshComponent)))