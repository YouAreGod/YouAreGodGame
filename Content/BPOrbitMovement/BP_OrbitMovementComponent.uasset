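; Actor component that moves its owner along gravitational orbits around BP_GravityMassComponent bodies.
; A constructed BP_Orbit object does the math and sets the start velocity, optionally circularized or velocity-matched.
; Each tick runs Kinematic (all masses, optional substeps), Kepler (analytic) or Blend (kinematic step snapped to orbit distance), dropping to Kinematic during input acceleration.
; Swept moves zero velocity on hits, and debug trails and orbit splines visualize paths.
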(event `self.ReceiveBeginPlay`
  (`self.InitializeOrbitMovement` false)
  (if (and (!= (`/Game/BPOrbitMovement/Lib/BP_Orbit.GravityMassOrbiting` (`self.Orbit`)) null) (`self.DrawOrbitOnBeginPlay`))
    (`self.DrawOrbitSpline` (`self.NumOfSplinePoints`))))

(event `self.ReceiveTick`
  (params (DeltaSeconds :type "Float (single-precision)"))
  (`self.OrbitTick` DeltaSeconds))

(fn `AddAllGravityMassesInScene`
  (bind _outactors (`GameplayStatics.GetAllActorsOfClass` "/Script/Engine.Actor"))
  (for _array_element _outactors
    (`KismetArrayLibrary.Array_AddUnique` (`self.GravityMassArray`) (`KismetArrayLibrary.Array_Get` (`Actor.K2_GetComponentsByClass` _array_element "/Game/BPOrbitMovement/BP_GravityMassComponent.BP_GravityMassComponent_C"))))
  (`KismetArrayLibrary.Array_RemoveItem` (`self.GravityMassArray`) null)
  (return))

(fn `BlendedTick`
  (params (DeltaTime :type "Float (double-precision)"))
  (locals (OldVel :type "Vector Structure") (RelAdjustedDelta :type "Vector Structure") (NewRelPos :type "Vector Structure") (NewWorldPos :type "Vector Structure"))
  (bind _returnvalue (`self.GetOwner`))
  (bind _orbit (`self.Orbit`))
  (`/Game/BPOrbitMovement/Lib/BP_Orbit.UpdateTimeSincePeriapsisIterator` (`self.Orbit`) DeltaTime)
  (set `local.OldVel` (`self.Velocity`))
  (`/Game/BPOrbitMovement/Lib/BP_Orbit.UpdateGravityOnlyFromMassOrbiting` (`self.Orbit`))
  ;[1 1 1] Calculate the correct velocity and kinematically obtain the PositionDelta
  (`self.UpdateKeplerVelocity`)
  (bind _newposdelta (`/Game/BPOrbitMovement/Lib/BP_Orbit.CalculateNewPositionDeltaKinematically` (`self.Orbit`) DeltaTime (`local.OldVel`) (`self.Velocity`)))
  (set `local.RelAdjustedDelta` _newposdelta)
  (bind _orbittype (`/Game/BPOrbitMovement/Lib/BP_Orbit.GetOrbitType` (`self.Orbit`)))
  (switch `/Game/BPOrbitMovement/Lib/BP_OrbitType` _orbittype
    (:`NewEnumerator0`
      ;[1 1 1] Based on where we ended up, find the 'correct' distance
      (bind _trueanomaly (`/Game/BPOrbitMovement/Lib/BP_Orbit.GetTrueAnomalyAtLocation` (`self.Orbit`) (+ (`Actor.K2_GetActorLocation` (`self.GetOwner`)) (`local.RelAdjustedDelta`)) :!label _label))
      (bind _distance (`/Game/BPOrbitMovement/Lib/BP_Orbit.GetDistance` (`self.Orbit`) _trueanomaly 0.0))
      ;[1 1 1] Obtain a relative position value based on the GravityMass orbiting
      (bind _relativelocation (`/Game/BPOrbitMovement/Lib/BP_Orbit.GetRelativeToMassLocation` (`self.Orbit`)))
      (bind _output_get (set `local.NewRelPos` (* (`/Game/BPOrbitMovement/Lib/BP_Orbit.UnsafeNormal` (`self.Orbit`) (+ _relativelocation (`local.RelAdjustedDelta`))) _distance)))
      (set `local.NewWorldPos` (+ _output_get (`Actor.K2_GetActorLocation` (`self.GetOwner` (`/Game/BPOrbitMovement/Lib/BP_Orbit.GravityMassOrbiting` (`self.Orbit`)))))))
    (:`NewEnumerator1`
      (goto _label))
    (:`NewEnumerator2`
      (goto _label))
    (:`NewEnumerator3`
      ;[1 1 1] Obtain a relative position value based on the GravityMass orbiting
      (bind _relativelocation_2 (`/Game/BPOrbitMovement/Lib/BP_Orbit.GetRelativeToMassLocation` (`self.Orbit`) :!label _label_2))
      (bind _output_get_2 (set `local.NewRelPos` (+ _relativelocation_2 (`local.RelAdjustedDelta`))))
      ;[1 1 1] Need to check if we are at 0 velocity and need to switch directions.
      (`/Game/BPOrbitMovement/Lib/BP_Orbit.CalculateNewVelocityDeltaKinematically` _orbit DeltaTime (0.0 0.0 0.0))
      (set `local.NewWorldPos` (+ _output_get_2 (`Actor.K2_GetActorLocation` (`self.GetOwner` (`/Game/BPOrbitMovement/Lib/BP_Orbit.GravityMassOrbiting` _orbit))))))
    (:`NewEnumerator4`
      (goto _label_2))
    (:`NewEnumerator5`
      (goto _label_2)))
  ;[1 1 1] Debug trails
  (if (`self.bDrawDebugTrails`)
    (`KismetSystemLibrary.DrawDebugLine` (`Actor.K2_GetActorLocation` _returnvalue) (`local.NewWorldPos`) (`self.TrailColor`) (`self.TrailTimeLength`) (`self.TrailThinkness`)))
  (bind _sweephitresult (`Actor.K2_SetActorLocation` _returnvalue (`local.NewWorldPos`) true false))
  (if (`GameplayStatics.BreakHitResult` _sweephitresult)
    (`self.HandleAHit` _sweephitresult))
  (`/Game/BPOrbitMovement/Lib/BP_Orbit.ClearKepplerOrbitUpdateVars` (`self.Orbit`)))

(fn `DrawOrbitSpline`
  (params (Points :type Integer))
  (returns (BP_OrbitSpline :type "/Game/BPOrbitMovement/Lib/BP_OrbitSpline Object Reference"))
  (locals (NumOfPoints :type Integer) (SplinePointArray :type "Array of Vector Structure") (IterationStep :type "Float (double-precision)") (TempBPSpline :type "/Game/BPOrbitMovement/Lib/BP_OrbitSpline Object Reference") (StartIteration :type "Float (double-precision)") (EndIteration :type "Float (double-precision)"))
  (bind _orbit (`self.Orbit`))
  (bind _splinepointarray (`local.SplinePointArray`))
  (set `local.NumOfPoints` Points)
  (bind _returnvalue (`|SpawnActorFromClass` "/Game/BPOrbitMovement/Lib/BP_OrbitSpline.BP_OrbitSpline_C" (`Actor.GetTransform` (`self.GetOwner`)) "Undefined" "OverrideRootScale" (`self.GetOwner`) 1.0 "/Game/ExampleContent/Props/Shape_Cylinder.Shape_Cylinder"))
  (set `local.TempBPSpline` _returnvalue)
  ;[1 1 1] First make an array of points for the spline, then add the points to the spline
  (`|ExecutionSequence`
    (:`then_0`
      (bind _orbittype (`/Game/BPOrbitMovement/Lib/BP_Orbit.GetOrbitType` (`self.Orbit`)))
      (switch `/Game/BPOrbitMovement/Lib/BP_OrbitType` _orbittype
        (:`NewEnumerator0`
          (set `local.IterationStep` (/ (`/Game/BPOrbitMovement/Lib/BP_Orbit.TWO_PI` (`self.Orbit`)) (`KismetMathLibrary.Conv_IntToDouble` (`local.NumOfPoints`))))
          (`SplineComponent.SetClosedLoop` (`/Game/BPOrbitMovement/Lib/BP_OrbitSpline.Spline` (`local.TempBPSpline`)) true true)
          (for _index (range (`local.NumOfPoints`))
            (bind _returnvalue_2 (* _index (`local.IterationStep`)))
            (bind _newtrueanomaly (`/Game/BPOrbitMovement/Lib/BP_Orbit.GetTrueAnomalyFromEccentricAnomaly` (`self.Orbit`) _returnvalue_2))
            (bind _position (`/Game/BPOrbitMovement/Lib/BP_Orbit.GetRelativePositionFromTrueAnomaly` (`self.Orbit`) _newtrueanomaly _returnvalue_2))
            (`KismetArrayLibrary.Array_Add` (`local.SplinePointArray`) (+ _position (`Actor.K2_GetActorLocation` (`self.GetOwner` (`/Game/BPOrbitMovement/Lib/BP_Orbit.GravityMassOrbiting` (`self.Orbit`))))))))
        (:`NewEnumerator1`
          (bind _eccentric_anomaly (`/Game/BPOrbitMovement/Lib/BP_Orbit.GetEccentricAnomaly` (`self.Orbit`)))
          ;[1 1 1] Set the start and end location of the spline by looking at its current position and propagating backwards and forwards
          (bind _output_get (set `local.StartIteration` (- _eccentric_anomaly (`self.LengthMultiplier`))))
          (bind _output_get_2 (set `local.EndIteration` (+ _eccentric_anomaly (`self.LengthMultiplier`))))
          ;[1 1 1] Devide the length of the anomaly to cover by number of points
          (set `local.IterationStep` (/ (- _output_get_2 _output_get) (`KismetMathLibrary.Conv_IntToDouble` (`local.NumOfPoints`))))
          (for _index_2 (range (`local.NumOfPoints`))
            (bind _returnvalue_3 (+ (* _index_2 (`local.IterationStep`)) (`local.StartIteration`)))
            (bind _newtrueanomaly_2 (`/Game/BPOrbitMovement/Lib/BP_Orbit.GetTrueAnomalyFromEccentricAnomaly` _orbit _returnvalue_3))
            (bind _position_2 (`/Game/BPOrbitMovement/Lib/BP_Orbit.GetRelativePositionFromTrueAnomaly` _orbit _newtrueanomaly_2 _returnvalue_3))
            (`KismetArrayLibrary.Array_Add` (`local.SplinePointArray`) (+ _position_2 (`Actor.K2_GetActorLocation` (`self.GetOwner`))))))
        (:`NewEnumerator2`
          (bind _eccentric_anomaly_2 (`/Game/BPOrbitMovement/Lib/BP_Orbit.GetEccentricAnomaly` (`self.Orbit`)))
          ;[1 1 1] Set the start and end location of the spline by looking at its current position and propagating backwards and forwards
          (bind _output_get_3 (set `local.StartIteration` (- _eccentric_anomaly_2 (`self.LengthMultiplier`))))
          (bind _output_get_4 (set `local.EndIteration` (+ _eccentric_anomaly_2 (`self.LengthMultiplier`))))
          ;[1 1 1] Devide the length of the anomaly to cover by number of points
          (set `local.IterationStep` (/ (- _output_get_4 _output_get_3) (`KismetMathLibrary.Conv_IntToDouble` (`local.NumOfPoints`))))
          (for _index_3 (range (`local.NumOfPoints`))
            (bind _returnvalue_4 (+ (* _index_3 (`local.IterationStep`)) (`local.StartIteration`)))
            (bind _newtrueanomaly_3 (`/Game/BPOrbitMovement/Lib/BP_Orbit.GetTrueAnomalyFromEccentricAnomaly` (`self.Orbit`) _returnvalue_4))
            (bind _position_3 (`/Game/BPOrbitMovement/Lib/BP_Orbit.GetRelativePositionFromTrueAnomaly` (`self.Orbit`) _newtrueanomaly_3 _returnvalue_4))
            (`KismetArrayLibrary.Array_Add` (`local.SplinePointArray`) (+ _position_3 (`Actor.K2_GetActorLocation` (`self.GetOwner` (`/Game/BPOrbitMovement/Lib/BP_Orbit.GravityMassOrbiting` (`self.Orbit`))))))))))
    (:`then_1`
      (`SplineComponent.SetSplinePoints` (`/Game/BPOrbitMovement/Lib/BP_OrbitSpline.Spline` (`local.TempBPSpline`)) _splinepointarray "World" true)
      (for _index_4 (range (`KismetArrayLibrary.Array_Length` _splinepointarray))
        (`SplineComponent.SetSplinePointType` (`/Game/BPOrbitMovement/Lib/BP_OrbitSpline.Spline` (`local.TempBPSpline`)) _index_4 "Curve" true))
      (`/Game/BPOrbitMovement/Lib/BP_OrbitSpline.DrawStaticMeshes` (`local.TempBPSpline`))
      (return (`local.TempBPSpline`)))))

(fn `HandleAHit`
  (params (Hit :type "HitResult Structure"))
  (set `/Game/BPOrbitMovement/Lib/BP_Orbit.OrbitVelocity` (0.0 0.0 0.0) (`self.Orbit`))
  (set `self.Velocity` (0.0 0.0 0.0)))

(fn `InitializeOrbitMovement`
  (params (DontCheckMatchVel :type Boolean))
  (set `self.SceneCompToUpdate` (`Actor.K2_GetRootComponent` (`self.GetOwner`)))
  (if (== (`KismetArrayLibrary.Array_Length` (`self.GravityMassArray`)) 0)
    (`self.AddAllGravityMassesInScene`))
  (set `self.MovementCompArray` (`Actor.K2_GetComponentsByClass` (`self.GetOwner`) "/Script/Engine.PawnMovementComponent"))
  (set `self.CurrentMovementPhysicsType` (`self.MovementPhysicsType`))
  ;[1 1 1] Construct and make a reference to the component's 'Orbit' class
  (bind _returnvalue (`|GenericCreateObject` "/Game/BPOrbitMovement/Lib/BP_Orbit.BP_Orbit_C" (`self.GetOwner`)))
  (set `self.Orbit` _returnvalue)
  ;[1 1 1] Setup Parent Actor and OrbitComponent variables in the Orbit class object
  (set `/Game/BPOrbitMovement/Lib/BP_Orbit.ParentActor` (`self.GetOwner`) (`self.Orbit`))
  (set `/Game/BPOrbitMovement/Lib/BP_Orbit.ParentOrbitComponent` self (`self.Orbit`))
  ;[1 1 1] Sets up the initial orbit based on StartVelocity, StartDirection, StartCircularized, etc
  (`self.SetupStartingOrbit` DontCheckMatchVel)
  ;[1 1 1] Set a random color for the debug trail lines if desired
  (if (`self.RandomColor`)
    (set `self.TrailColor` (make `LinearColor` (`KismetMathLibrary.RandomFloatInRange` 0.0 1.0) (`KismetMathLibrary.RandomFloatInRange` 0.0 1.0) (`KismetMathLibrary.RandomFloatInRange` 0.0 1.0) 1.0))))

(fn `OrbitTick`
  (params (DeltaTime :type "Float (double-precision)"))
  (locals (DTime :type "Float (double-precision)") (bLastSubsteb :type Boolean) (SubstepTimeIterator :type "Float (double-precision)") (SubStepDeltaTime :type "Float (double-precision)") (SubStepIterator :type "Float (double-precision)") (NextSubstepIteratorValue :type "Float (double-precision)"))
  (bind _movementcomparray (`self.MovementCompArray`))
  (set `self.InputAcceleration` (0.0 0.0 0.0))
  (if (`self.IncorporateOtherMoveCompInput`)
    ;[1 1 1] Incorporate other movement components input acceleration into orbitmovement component
    (if (> (`KismetArrayLibrary.Array_Length` _movementcomparray) 0)
      (for _array_element _movementcomparray
        (if (`self.IsActive` _array_element)
          (set `self.InputAcceleration` (+ (`PawnMovementComponent.GetLastInputVector` _array_element) (`self.InputAcceleration`)))
          (set `MovementComponent.Velocity` (`self.Velocity`) _array_element)))))
  (set `local.DTime` DeltaTime)
  ;[1 1 1] Switch back to starting physics mode if Acceleration is complete and non-kinematic physics mode was selected.
  (if (and (`self.IsCurrentlyAccelerating`) (== (`self.InputAcceleration`) (0.0 0.0 0.0) :`ErrorTolerance` 0.0))
    (`/Game/BPOrbitMovement/Lib/BP_Orbit.InitNewOrbit` (`self.Orbit`) (`Actor.K2_GetActorLocation` (`self.GetOwner`)) (`self.Velocity`))
    (set `self.CurrentMovementPhysicsType` (`self.MovementPhysicsType`))
    (set `self.IsCurrentlyAccelerating` false))
  ;[1 1 1] Use custom Tick time if desired.
  (if (not (`self.bRealTime`))
    (set `local.DTime` (`self.SimulatedTimeStep`)))
  (set `self.IsCurrentlyAccelerating` (!= (`self.InputAcceleration`) (0.0 0.0 0.0) :`ErrorTolerance` 0.0))
  (switch `/Game/BPOrbitMovement/Lib/BP_SimulationBehaviorType` (`self.CurrentMovementPhysicsType`)
    (:`NewEnumerator0`
      (if (and (`self.bSubStepKinematicPhysics`) (> (`local.DTime`) (`self.SubstepTimeStep`))) :!label _label
        ;[1 1 1] Physics Substepping
        (set `local.bLastSubsteb` false)
        (set `local.SubstepTimeIterator` 0.0)
        (set `local.SubStepDeltaTime` (`self.SubstepTimeStep`))
        (set `local.SubStepIterator` 1.0)
        (while (not (`local.bLastSubsteb`))
          (set `local.NextSubstepIteratorValue` (+ (`local.SubStepDeltaTime`) (`local.SubstepTimeIterator`)))
          (if (or (> (`local.NextSubstepIteratorValue`) (`local.DTime`)) (== (`local.SubStepIterator`) (`self.MaxSubstepIterations`)))
            (set `local.SubStepDeltaTime` (- (`local.DTime`) (`local.SubstepTimeIterator`)))
            (set `local.SubstepTimeIterator` (+ (`local.SubstepTimeIterator`) (`local.SubStepDeltaTime`)))
            (set `local.bLastSubsteb` true)
            (else
              (set `local.SubstepTimeIterator` (`local.NextSubstepIteratorValue`))))
          (`self.UpdateKinematicPosition` (`local.SubStepDeltaTime`))
          (`/Game/BPOrbitMovement/Lib/BP_Orbit.ClearOrbitUpdateVars` (`self.Orbit`))
          (set `local.SubStepIterator` (+ (`local.SubStepIterator`) 1.0)))
        (else
          (`self.UpdateKinematicPosition` (`local.DTime`))
          ;[1 1 1] Clear all orbit parameters when in kinematic mode because kinematic orbits slightly change each frame
          (`/Game/BPOrbitMovement/Lib/BP_Orbit.ClearOrbitUpdateVars` (`self.Orbit`)))))
    (:`NewEnumerator1`
      ;[1 1 1] Use kinematic physics mode if there is a user inputted acceleration.
      (if (`self.IsCurrentlyAccelerating`)
        (set `self.CurrentMovementPhysicsType` "NewEnumerator0")
        (goto _label)
        (else
          (`self.UpdateKeplerPosition` (`local.DTime`)))))
    (:`NewEnumerator2`
      (if (`self.IsCurrentlyAccelerating`)
        (set `self.CurrentMovementPhysicsType` "NewEnumerator0")
        (goto _label)
        (else
          (`self.BlendedTick` (`local.DTime`)))))))

(fn `SetupStartingOrbit`
  (params (DontCheckParentVelocity :type Boolean))
  (locals (TempStartVelocity :type "Vector Structure") (TempCircularOrbitStartDirection :type "Vector Structure") (DontCheckMathchVelocity :type Boolean) (MatchVelCheck :type Boolean))
  (bind _gravitymasstoorbit (`self.GravityMassToOrbit`))
  (bind _returnvalue (`Actor.GetComponentByClass` _gravitymasstoorbit "/Game/BPOrbitMovement/BP_GravityMassComponent.BP_GravityMassComponent_C"))
  ;[1 1 1] Needed for infitite recursion checking
  (if DontCheckParentVelocity
    (set `local.MatchVelCheck` false)
    (else
      (set `local.MatchVelCheck` (`self.bMatchGravityMassVelOnStart`))))
  (set `local.TempCircularOrbitStartDirection` (`self.CircularOrbitDirectionToStart`))
  (set `local.TempStartVelocity` (`self.StartVelocity`))
  (if (== _gravitymasstoorbit null)
    ;[1 1 1] Default the actor that this actor is orbiting to whatever GravityMass is having the largest influence
    (`/Game/BPOrbitMovement/Lib/BP_Orbit.SetGravityMassOrbitingToLargestInfluence` (`self.Orbit`) (`self.GravityMassArray`) :!label _label)
    (elif (== _returnvalue null)
      (goto _label)
      (else
        (`/Game/BPOrbitMovement/Lib/BP_Orbit.SetGravityMassOrbiting` (`self.Orbit`) _returnvalue))))
  (if (`self.StartVelocity in Local Space`)
    (set `local.TempStartVelocity` (`KismetMathLibrary.TransformDirection` (`Actor.GetTransform` (`self.GetOwner`)) (`local.TempStartVelocity`)))
    (set `local.TempCircularOrbitStartDirection` (`KismetMathLibrary.TransformDirection` (`Actor.GetTransform` (`self.GetOwner`)) (`local.TempCircularOrbitStartDirection`))))
  ;[1 1 1] Finds a start velocity based on circularized orbit and velocity matching options
  (bind _startingvelocity (`/Game/BPOrbitMovement/Lib/BP_Orbit.ComputeStartVelocity` (`self.Orbit`) (`local.MatchVelCheck`) (`self.StartCircularized`) (`local.TempStartVelocity`) (`local.TempCircularOrbitStartDirection`)))
  (bind _output_get (set `self.Velocity` _startingvelocity))
  ;[1 1 1] Need to not have infinite recursion while checking parent velocities
  (if (`local.MatchVelCheck`)
    ;[1 1 1] Initialize the orbit based on the starting parameters
    (`/Game/BPOrbitMovement/Lib/BP_Orbit.InitNewOrbit` (`self.Orbit`) (`Actor.K2_GetActorLocation` (`self.GetOwner`)) _output_get)
    (set `self.HasInit` true)))

(fn `TransferVelocityToOtherMovementComponent`
  (bind _returnvalue (`Actor.K2_GetComponentsByClass` (`self.GetOwner`) "/Script/Engine.MovementComponent"))
  (if (!= (`KismetArrayLibrary.Array_Length` _returnvalue) 0)
    (set `MovementComponent.Velocity` (`self.Velocity`) (`KismetArrayLibrary.Array_Get` _returnvalue))
    (set `self.Velocity` (0.0 0.0 0.0))
    (return)
    (else
      (return))))

(fn `UpdateKeplerPosition`
  (params (DeltaTime :type "Float (double-precision)"))
  (locals (NewPos :type "Vector Structure") (Adjusted :type "Vector Structure"))
  (bind _orbit (`self.Orbit`))
  ;[1 1 1] Add deltaTime so we know where in the orbit the actor should be
  (`/Game/BPOrbitMovement/Lib/BP_Orbit.UpdateTimeSincePeriapsisIterator` (`self.Orbit`) DeltaTime)
  (`self.UpdateKeplerVelocity`)
  ;[1 1 1] Calculates the position based on TimeSincePeriapsis, relative to the GravityMass orbiting
  (bind _new_position (`/Game/BPOrbitMovement/Lib/BP_Orbit.CalculatePositionFromTimeSincePeriapsisKeppler` _orbit (`/Game/BPOrbitMovement/Lib/BP_Orbit.TimeSincePeriapsisIterator` _orbit)))
  (bind _output_get (set `local.NewPos` (+ _new_position (`Actor.K2_GetActorLocation` (`self.GetOwner` (`/Game/BPOrbitMovement/Lib/BP_Orbit.GravityMassOrbiting` (`self.Orbit`)))))))
  ;[1 1 1] Debug trails
  (if (`self.bDrawDebugTrails`)
    (`KismetSystemLibrary.DrawDebugLine` (`Actor.K2_GetActorLocation` (`self.GetOwner`)) _output_get (`self.TrailColor`) (`self.TrailTimeLength`) (`self.TrailThinkness`)))
  (bind _sweephitresult (`Actor.K2_SetActorLocation` (`self.GetOwner`) _output_get true false))
  (if (`GameplayStatics.BreakHitResult` _sweephitresult)
    (`self.HandleAHit` _sweephitresult))
  ;[1 1 1] Clear orbital parameters that change each frame. I.e. True Anomaly
  (`/Game/BPOrbitMovement/Lib/BP_Orbit.ClearKepplerOrbitUpdateVars` (`self.Orbit`)))

(fn `UpdateKeplerVelocity`
  (bind _newvelocity (`/Game/BPOrbitMovement/Lib/BP_Orbit.UpdateOrbitVelocityKeppler` (`self.Orbit`)))
  (bind _output_get (set `self.Velocity` (+ _newvelocity (`/Game/BPOrbitMovement/Lib/BP_Orbit.GetGravityMassVelocity` (`self.Orbit`)))))
  (if (`SceneComponent.IsSimulatingPhysics` (`self.SceneCompToUpdate`) "None")
    (bind _asprimitive_component (cast `PrimitiveComponent` (`self.SceneCompToUpdate`)))
    (`PrimitiveComponent.SetPhysicsLinearVelocity` _asprimitive_component _output_get false "None")))

(fn `UpdateKinematicPosition`
  (params (DeltaTime :type "Float (double-precision)"))
  (locals (OldVel :type "Vector Structure"))
  (bind _returnvalue (`Actor.K2_GetActorLocation` (`self.GetOwner`)))
  (`/Game/BPOrbitMovement/Lib/BP_Orbit.UpdateTimeSincePeriapsisIterator` (`self.Orbit`) DeltaTime)
  ;[1 1 1] Find and set the acceleration due to gravity for each GravityMass in the scene
  (`/Game/BPOrbitMovement/Lib/BP_Orbit.UpdateGravity` (`self.Orbit`) (`self.GravityMassArray`))
  (set `local.OldVel` (`self.Velocity`))
  (`self.UpdateKinematicVelocity` DeltaTime)
  ;[1 1 1] Find this frame's position difference
  (bind _newposdelta (`/Game/BPOrbitMovement/Lib/BP_Orbit.CalculateNewPositionDeltaKinematically` (`self.Orbit`) DeltaTime (`local.OldVel`) (`self.Velocity`)))
  ;[1 1 1] Debug trails
  (if (`self.bDrawDebugTrails`)
    (bind _returnvalue_2 (+ _newposdelta _returnvalue))
    (`KismetSystemLibrary.DrawDebugLine` _returnvalue _returnvalue_2 (`self.TrailColor`) (`self.TrailTimeLength`) (`self.TrailThinkness`)))
  ;[1 1 1] Set actor to the new location
  (bind _sweephitresult (`Actor.K2_SetActorLocation` (`self.GetOwner`) _returnvalue_2 true false))
  (if (`GameplayStatics.BreakHitResult` _sweephitresult)
    (`self.HandleAHit` _sweephitresult)))

(fn `UpdateKinematicVelocity`
  (params (DeltaTime :type "Float (double-precision)"))
  (bind _velocitydelta (`/Game/BPOrbitMovement/Lib/BP_Orbit.CalculateNewVelocityDeltaKinematically` (`self.Orbit`) DeltaTime (+ (`self.AdditionalWorldAccel`) (* (`self.InputAcceleration`) (`self.AccelerationMultiplier`)))))
  (set `self.Velocity` (+ _velocitydelta (`self.Velocity`)))
  (if (`SceneComponent.IsSimulatingPhysics` (`self.SceneCompToUpdate`) "None")
    (bind _asprimitive_component (cast `PrimitiveComponent` (`self.SceneCompToUpdate`)))
    (`PrimitiveComponent.AddImpulse` _asprimitive_component _velocitydelta "None" true)))